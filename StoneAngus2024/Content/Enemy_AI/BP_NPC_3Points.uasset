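; Guard NPC that patrols a fixed route and catches pawns it sees.
; GuardPatrol uses AIMoveTo through the PatrolLocation array, idles for a random pause on arrival, then calls itself, with an index that wraps at four despite the asset's "3Points" name.
; PawnSensing sightings halt movement, play a fade-to-black sequence and briefly show the W_Caught widget.
; All widgets are then removed and the patrol resumes after timed delays.
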(event OnSeePawn(PawnSensing)
  (params (Pawn :type Pawn%20Object%20Reference))
  ;[1 1 1] Player Caught
  (Pawn|Components|CharacterMovement|DisableMovement (Variables|Character|GetCharacterMovement))
  (Components|Animation|PlayAnimation (Variables|Character|GetMesh) "/Game/Characters/Mannequins/Animations/Quinn/MF_Idle.MF_Idle" false)
  (Utilities|FlowControl|Delay 0.2)
  (bind _returnvalue (Sequencer|Player|CreateLevelSequencePlayer "/Game/Sequences/Fade_To_Black.Fade_To_Black"))
  (Sequencer|Player|Play _returnvalue :!class /Script/MovieScene.MovieSceneSequencePlayer)
  (Utilities|FlowControl|Delay 2.0)
  (bind _returnvalue_2 (UserInterface|CreateWidget "/Game/Widgets/W_Caught.W_Caught_C"))
  (UserInterface|Viewport|AddtoViewport _returnvalue_2 0)
  (Utilities|FlowControl|Delay 2.0)
  (Viewport|RemoveAllWidgets)
  (Utilities|FlowControl|Delay 2.0)
  (Pawn|Components|CharacterMovement|SetMovementMode (Variables|Character|GetCharacterMovement) "MOVE_Walking" 0)
  (Components|Animation|PlayAnimation (Variables|Character|GetMesh) "/Game/Characters/Mannequins/Animations/Quinn/MF_Walk_Fwd.MF_Walk_Fwd" true)
  (CallFunction|GuardPatrol))

(event Custom|Guard%20Patrol
  ;[1 1 1] Enemy Patrol
  (Variables|/Script/Engine.CharacterMovementComponent|SetMaxWalkSpeed (Variables|Character|GetCharacterMovement) 6e+02)
  (AI|AIMoveTo self (Utilities|Array|Get(acopy) (Variables|Default|GetPatrol%20Location) (Variables|Default|GetLocation)) 0 5.0 false
    (:OnSuccess
      (Components|Animation|PlayAnimation (Variables|Character|GetMesh) "/Game/Characters/Mannequins/Animations/Quinn/MF_Idle.MF_Idle" false)
      (Utilities|FlowControl|Delay (Math|Random|RandomFloatinRange 1.0 2.0))
      (CallFunction|GuardPatrol)
      (Components|Animation|PlayAnimation (Variables|Character|GetMesh) "/Game/Characters/Mannequins/Animations/Quinn/MF_Walk_Fwd.MF_Walk_Fwd" true)
      (Math|Integer|IncrementInt (Variables|Default|GetLocation)
        (:%20%20
          (if (== (Variables|Default|GetLocation) 4)
            (Variables|Default|SetLocation 0)))))))

(event EventBeginPlay
  ;[1 1 1] Enemy Patrol
  (CallFunction|GuardPatrol))

(fn ConstructionScript)